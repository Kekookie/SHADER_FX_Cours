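; Firework rocket actor that shows a configurable Niagara rocket with trails, then explodes into a radial burst.
; Construction sets its lifespan and feeds scale, colors and a dynamic sprite material to the rocket system, or hides it.
; BeginPlay attaches a Niagara trail per TrailEffects entry (sparks, smoke or spiral) with its own parameters.
; Tick compares time since creation to deactivate trails after RocketLifespan, then spawns NS_Radial_Burst at the collider after ExplosionDelay.
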(event `self.ReceiveBeginPlay`
  (`self.SetNiagaraTrails`))

(event `self.ReceiveTick`
  (params (DeltaSeconds :type "Float (single-precision)"))
  (if (and (> (`self.GetGameTimeSinceCreation`) (`self.RocketLifespan`)) (`self.IsTrailActive`))
    (set `self.IsTrailActive` false)
    (`self.DeactivateTrails`))
  (if (and (> (`self.GetGameTimeSinceCreation`) (+ (`self.ExplosionDelay`) (`self.RocketLifespan`))) (`self.IsUnexploded`))
    (`self.ExplodeRocket`)
    (set `self.IsUnexploded` false)))

(fn `DeactivateTrails`
  (for _array_element (`self.TrailReferences`)
    (`ActorComponent.Deactivate` _array_element)))

(fn `ExplodeRocket`
  (`NiagaraFunctionLibrary.SpawnSystemAtLocation` "/Game/StarterContent/Particles/Niagara_System/NS_Radial_Burst.NS_Radial_Burst" (`SceneComponent.K2_GetComponentLocation` (`self.C_Collider`))))

(fn `SetNiagaraRocketProperties`
  (bind _niagara_rocket (`self.Niagara_Rocket`))
  (if (`self.RocketVisible`)
    (`NiagaraComponent.SetVariableFloat` _niagara_rocket "Lifespan" (`self.RocketLifespan`))
    (`NiagaraComponent.SetVariableFloat` _niagara_rocket "RocketSpriteScale" (`self.RocketScale`))
    (`NiagaraComponent.SetVariableLinearColor` _niagara_rocket "StartColor" (`self.RocketStartColor`))
    (`NiagaraComponent.SetVariableLinearColor` _niagara_rocket "EndColor" (`self.RocketEndColor`))
    (bind _returnvalue (`KismetMaterialLibrary.CreateDynamicMaterialInstance` "/Game/Arts/Fireworks_VFX_Test_Rendu/Material/M_Rocket.M_Rocket"))
    (`MaterialInstanceDynamic.SetTextureParameterValue` _returnvalue "ParticleTexture" (`self.RocketSprite`))
    (`NiagaraComponent.SetVariableMaterial` _niagara_rocket "SpriteMaterialInst" _returnvalue)
    (else
      (`SceneComponent.SetVisibility` (`self.Niagara_Rocket`) false false))))

(fn `SetNiagaraTrails`
  (locals (TempNiagaraAsset :type "NiagaraSystem Object Reference" :default null) (TrailRef :type "NiagaraComponent Object Reference"))
  (for _array_element (`self.TrailEffects`)
    (bind (_type _densityscale _lenghtscale _spritescale _startcolor _endcolor) (break `/Game/Arts/Fireworks_VFX_Test_Rendu/Blueprints/S_Fireworks_TrailSettings` _array_element))
    (switch `/Game/Arts/Fireworks_VFX_Test_Rendu/Blueprints/E_Fireworks_TrailType` _type
      (:`NewEnumerator0`
        (set `local.TempNiagaraAsset` "/Game/Arts/Fireworks_VFX_Test_Rendu/Niagara/Trails/NS_Trail_SimpleSparks.NS_Trail_SimpleSparks"))
      (:`NewEnumerator1`
        (set `local.TempNiagaraAsset` "/Game/Arts/FX/Niagara_System/Smoke/NS_Smoke.NS_Smoke"))
      (:`NewEnumerator2`
        (set `local.TempNiagaraAsset` "/Game/Arts/Fireworks_VFX_Test_Rendu/Niagara/Trails/NS_Trail_Spiral.NS_Trail_Spiral")))
    (bind _returnvalue (`NiagaraFunctionLibrary.SpawnSystemAttached` (`local.TempNiagaraAsset`) (`self.C_Collider`) "None" (0.0 0.0 0.0) (struct) "KeepRelativeOffset"))
    (bind _output_get (set `local.TrailRef` _returnvalue))
    (`NiagaraComponent.SetVariableFloat` _output_get "TrailDuration" (`self.RocketLifespan`))
    (`NiagaraComponent.SetVariableFloat` (`local.TrailRef`) "TrailSpriteScale" _spritescale)
    (`NiagaraComponent.SetVariableFloat` (`local.TrailRef`) "TrailLengthScale" _lenghtscale)
    (`NiagaraComponent.SetVariableFloat` (`local.TrailRef`) "TrailDensityScale" _densityscale)
    (`NiagaraComponent.SetVariableLinearColor` (`local.TrailRef`) "StartColor" _startcolor)
    (`NiagaraComponent.SetVariableLinearColor` (`local.TrailRef`) "EndColor" _endcolor)
    (`KismetArrayLibrary.Array_Add` (`self.TrailReferences`) (`local.TrailRef`))))

(fn `UserConstructionScript`
  (`self.SetLifeSpan` (* (+ (`self.RocketLifespan`) (`self.ExplosionDelay`)) 2.0))
  (`self.SetNiagaraRocketProperties`))