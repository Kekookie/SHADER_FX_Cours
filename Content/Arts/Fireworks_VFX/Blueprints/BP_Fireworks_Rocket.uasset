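; Firework rocket actor that times its flight and explodes into a radial burst Niagara effect.
; Tick compares time since creation to RocketLifespan to hide the collider component once, then after ExplosionDelay spawns the burst at the collider's location.
; The IsUnexploded check is unconnected, so the burst respawns every tick until the actor expires.
; The construction script sets actor lifespan to twice the combined flight and delay time.
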(event `self.ReceiveTick`
  (params (DeltaSeconds :type "Float (single-precision)"))
  (if (and (> (`self.GetGameTimeSinceCreation`) (`self.RocketLifespan`)) (`self.IsTrailActive`))
    (set `self.IsTrailActive` false)
    (`SceneComponent.SetVisibility` (`self.C_Collider`) false false))
  (if (> (`self.GetGameTimeSinceCreation`) (+ (`self.ExplosionDelay`) (`self.RocketLifespan`)))
    (`self.ExplodeRocket`)
    (set `self.IsUnexploded` false)))

(fn `ExplodeRocket`
  (`NiagaraFunctionLibrary.SpawnSystemAtLocation` "/Game/StarterContent/Particles/Niagara_System/NS_Radial_Burst.NS_Radial_Burst" (`SceneComponent.K2_GetComponentLocation` (`self.C_Collider`))))

(fn `UserConstructionScript`
  (`self.SetLifeSpan` (* (+ (`self.RocketLifespan`) (`self.ExplosionDelay`)) 2.0)))