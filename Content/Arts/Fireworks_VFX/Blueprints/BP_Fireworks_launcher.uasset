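; Fireworks launcher actor that fires timed sequences of BP_Fireworks_Rocket actors, started by ShootRockets and halted by StopShooting.
; While active, Tick checks separate delays for the first sequence, between rockets and between repeats, optionally looping.
; Each rocket spawns at an offset with the launcher's appearance and timing settings, then gets physics velocity within a random cone around actor up.
; The construction script applies the launcher's mesh, transform and visibility.
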(event `self.ReceiveBeginPlay`
  (set `self.IsArmed` true))

(event `self.ReceiveTick`
  (params (DeltaSeconds :type "Float (single-precision)"))
  (if (and (`self.IsActive`) (`self.CheckLauncherTimer`))
    (`self.ShootSingleRocket`)
    (`self.UpdateSequence`)))

(fn `CheckLauncherTimer`
  (returns (CanLaunch :type Boolean))
  (locals (TempDelayTime :type "Float (double-precision)"))
  ;[1 1 1] 1st rocket
  (if (== (`self.CurrentRocketIndex`) 0)
    (if (`self.IsLooping`)
      ;[1 1 1] >= 2nd loop
      (set `local.TempDelayTime` (`self.DelayBetweenSequences`))
      (else
        ;[1 1 1] 1st loop
        (set `local.TempDelayTime` (`self.InitialSequenceDelay`))))
    (else
      ;[1 1 1] >= 2nd rocket
      (set `local.TempDelayTime` (`self.DelayBetweenRockets`))))
  (return (>= (`GameplayStatics.GetTimeSeconds`) (+ (`self.LastLaunchTime`) (`local.TempDelayTime`)))))

(fn `SetLauncherMesh`
  (bind _c_launchermesh (`self.C_LauncherMesh`))
  (`StaticMeshComponent.SetStaticMesh` _c_launchermesh (`self.LauncherMesh`))
  (`SceneComponent.K2_SetRelativeTransform` _c_launchermesh (`self.LauncherTransform`) false false)
  (`SceneComponent.SetVisibility` _c_launchermesh (`self.LauncherVisibility`) false))

(fn `ShootRockets`
  (if (`self.IsArmed`)
    (set `self.LastLaunchTime` (`GameplayStatics.GetTimeSeconds`))
    (set `self.IsActive` true)
    (set `self.IsLooping` false)))

(fn `ShootSingleRocket`
  (if (`self.IsArmed`)
    (bind _returnvalue (`|SpawnActorFromClass` "/Game/Arts/Fireworks_VFX/Blueprints/BP_Fireworks_Rocket.BP_Fireworks_Rocket_C" (`KismetMathLibrary.MakeTransform` (+ (`self.K2_GetActorLocation`) (`KismetMathLibrary.TransformDirection` (`self.GetTransform`) (`self.LauncherPositionOffset`))) (`self.K2_GetActorRotation`)) "AlwaysSpawn" "MultiplyWithRoot" null (`self.RocketLifespan`) (`self.ExplosionDelay`) (`self.RocketVisible`) (`self.RocketSprite`) (`self.RocketStartColor`) (`self.RocketScale`) (`self.RocketEndColor`) (`self.RandomSpriteRotation`) (`self.TrailEffects`) null))
    (`PrimitiveComponent.SetPhysicsLinearVelocity` (`/Game/Arts/Fireworks_VFX/Blueprints/BP_Fireworks_Rocket.C_Collider` _returnvalue) (* (`KismetMathLibrary.RandomUnitVectorInConeInDegrees` (`self.GetActorUpVector`) (`self.RandomLaunchAngle`)) (`self.InitialRocketSpeed`)) false "None")
    (set `self.LastLaunchTime` (`GameplayStatics.GetTimeSeconds`))))

(fn `StopShooting`
  (set `self.IsActive` false))

(fn `UpdateSequence`
  (bind _result (`/Engine/EditorBlueprintResources/StandardMacros.IncrementInt` (`self.CurrentRocketIndex`))
    (:`  `
      (if (< _result (`self.NumberOfRocketsLaunched`))
        (return)
        (else
          (set `self.CurrentRocketIndex` 0)
          (if (`self.SequenceLoops`)
            (set `self.IsLooping` true)
            (else
              (set `self.IsActive` false)))
          (return))))))

(fn `UserConstructionScript`
  (`self.SetLauncherMesh`))